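; Decay Grenade skill pickup that attaches to the player's left hand on overlap and becomes their current skill.
; Activation checks mana and cooldown, spawns a grenade copy at the player, then shows an explosion two seconds later.
; Enemies overlapping the held actor's own sphere lose half their health, which regenerates gradually after a delay if they survive.
; Recursive delays tick cooldown and mana-draining duration, but the StopSkill event they reach is empty.
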(event OnComponentBeginOverlap(Sphere)
  (params (OverlappedComponent :type Primitive%20Component%20Object%20Reference) (OtherActor :type Actor%20Object%20Reference) (OtherComp :type Primitive%20Component%20Object%20Reference) (OtherBodyIndex :type Integer) (bFromSweep :type Boolean) (SweepResult :type Hit%20Result%20Structure%20%28by%20ref%29))
  ;[1 1 1] Picking up the decay grenade
  (bind _asbp_third_person_character (Utilities|Casting|CastToBP_ThirdPersonCharacter OtherActor))
  (bind _output_get (Variables|Default|SetAs%20BP%20Third%20Person%20Character _asbp_third_person_character)) ; We'll need this for mana, ammo, and other checks
  (Variables|/Game/ThirdPerson/Blueprints/BP_ThirdPersonCharacter.BP_ThirdPersonCharacter_C|GetCurrentSKill _output_get
    (:then
      (Development|PrintString "You're already holding a skill!"))
    (:else
      (Variables|/Game/ThirdPerson/Blueprints/BP_ThirdPersonCharacter.BP_ThirdPersonCharacter_C|SetCurrentSKill _output_get self)
      (Transformation|AttachComponentToComponent (Variables|/Script/Engine.Character|GetMesh _output_get) "hand_lSocket" "SnapToTarget" "SnapToTarget" "SnapToTarget" true) ; attach this skill to the player's left hand
      (Development|PrintString "Holding Decay Grenade now!")
      (Rendering|SetVisibility (Variables|Default|GetGrenade) false false)
      (Collision|SetCollisionEnabled (Variables|Default|GetGrenade) "NoCollision"))))

(event OnComponentHit(Grenade)
  (params (HitComponent :type Primitive%20Component%20Object%20Reference) (OtherActor :type Actor%20Object%20Reference) (OtherComp :type Primitive%20Component%20Object%20Reference) (NormalImpulse :type Vector :default "0, 0, 0") (Hit :type Hit%20Result%20Structure%20%28by%20ref%29))
  (if (Variables|Default|GetSkill%20is%20Active)
    _))

(event OnComponentHit(Sphere)
  (params (HitComponent :type Primitive%20Component%20Object%20Reference) (OtherActor :type Actor%20Object%20Reference) (OtherComp :type Primitive%20Component%20Object%20Reference) (NormalImpulse :type Vector :default "0, 0, 0") (Hit :type Hit%20Result%20Structure%20%28by%20ref%29))
  (Utilities|Casting|CastToBP_DecayGrenade OtherActor))

(event OnComponentActivated(RadialForce)
  (params (Component :type Actor%20Component%20Object%20Reference) (bReset :type Boolean)))

(event Custom|Update%20Skill%20Duration
  ;[1 1 1] For every tenth of a second that this skill is active, reduce the number of remaining time on the skill.
  (if (Variables|Default|GetSkill%20is%20Active)
    (bind _output_get (Variables|Default|SetSkill%20Duration (- (Variables|Default|GetSkill%20Duration) 0.1)))
    (if (>= (Variables|Default|GetSkill%20Duration) 0.0) ; if true keep going\nelse, stop the skill
      (bind _hasmana (Default|UpdatePlayerStats (Variables|Default|GetAs%20BP%20Third%20Person%20Character) 0.0 -0.02 0.0))
      (if _hasmana ; if I have mana, keep going.\nelse, stop skill
        (Utilities|FlowControl|Delay 0.1)
        (Development|PrintString (Utilities|String|Append "DecayGrenade remaining duration is" (Utilities|String|ToString(Float) _output_get)) true true "(R=0.000000,G=0.660000,B=1.000000,A=1.000000)" 0.1)
        (CallFunction|UpdateSkillDuration)
        (else
          (CallFunction|StopSkill :!label _label)))
      (else
        (goto _label)))))

(event Custom|Stop%20Skill%20James
  ;[1 1 1] Let's turn off the skill, either because the skill has run out of time, or because we have ended it early, or if the player has run out of mana
  (if (Variables|Default|GetSkill%20is%20Active)
    (Variables|Default|SetSkill%20is%20Active false)
    (Variables|Default|SetSkill%20Cooldown (- 5.0 (Variables|Default|GetSkill%20Duration))) ; subtract whatever time the \nplayer still had for this effect
    (Variables|Default|SetSkill%20Duration 5.0) ; reset skill duration
    (Variables|Default|SetHoldCount 0)
    (CallFunction|UpdateSkillCooldown)
    (else
      (Development|PrintString "skill is already inactive"))))

(event Custom|Update%20Skill%20Cooldown%20James
  ;[1 1 1] As long as Cooldown is above zero, let's reduce that number and stop the player from starting up this skill again.
  (if (> (Variables|Default|GetSkill%20Cooldown) 0.0)
    (bind _output_get (Variables|Default|SetSkill%20Cooldown (- (Variables|Default|GetSkill%20Cooldown) 0.1)))
    (Utilities|FlowControl|Delay 0.1)
    (Development|PrintString (Utilities|String|Append "DecayGrenade cooldown is" (Utilities|String|ToString(Float) _output_get)) true true "(R=0.000000,G=0.660000,B=1.000000,A=1.000000)" 0.1)
    (CallFunction|UpdateSkillCooldownJames)))

(event Custom|Stop%20Skill)

(event Custom|Update%20Skill%20Cooldown)

(event Custom|CheckHealth
  ;[1 1 1] Checks to make sure enemy is still alive before adding health back
  (if (>= (Variables|/Game/AI_Blueprints/BP_Enemy_Base.BP_Enemy_Base_C|GetHealth (stale EventBeginSkill _asbp_enemy_base)) 0.0)
    (Variables|Default|SetAlive? true)
    (else
      (Variables|Default|SetAlive? false))))

(event EventHoldSkill
  ;[1 1 1] Optional Event for skills that you'd like to "hold down".
)

(event EventEndSkill
  ;[1 1 1] Optional, for skills that can be ended early.
)

(event EventBeginSkill
  (bind _returnvalue (Game|GetPlayerCharacter 0))
  ;[1 1 1] If the cooldown is at or below 0, we can start this skill!
  (bind _hasmana (Default|UpdatePlayerStats (Variables|Default|GetAs%20BP%20Third%20Person%20Character) 0.0 0.0 0.0))
  (if _hasmana ; if I have mana, keep going.\nelse, stop skill
    (Development|PrintString "Begin DG Skill 1")
    (if (<= (Variables|Default|GetSkill%20Cooldown) 0.0)
      (Variables|Default|SetSkill%20Cooldown 3.0)
      (Default|UpdatePlayerStats (Variables|Default|GetAs%20BP%20Third%20Person%20Character) 0.0 -0.1 0.0)
      (CallFunction|UpdateSkillCooldownJames)
      (Variables|Default|SetSkill%20is%20Active true)
      (CallFunction|UpdateSkillDuration)
      (Development|PrintString "Right click successful 2")
      (if (Variables|Default|GetSkill%20is%20Active) ; Checks if skill has\nbeen grabbed
        (bind _returnvalue_2 (Game|SpawnActorfromClass "BP_DecayGrenade_C" (Math|Transform|MakeTransform (Transformation|GetWorldLocation (Variables|/Script/Engine.Actor|GetRootComponent _returnvalue)) (Transformation|GetActorRotation _returnvalue) "1.000000,1.000000,1.000000") "AlwaysSpawn" "MultiplyWithRoot" 0 0)) ; Spawns grenade on action click being pressed
        (Development|PrintString "Spawned Grenade 3")
        (Utilities|FlowControl|Delay 2.0)
        (Effects|SpawnEmitteratLocation "/Game/Realistic_Starter_VFX_Pack_Vol2/Particles/Explosion/P_Explosion_Big_A.P_Explosion_Big_A" (Transformation|GetWorldLocation (Variables|/Script/Engine.Actor|GetRootComponent _returnvalue_2)) "0, 0, 0" "2.000000,2.000000,2.000000") ; Spawns explosion particles at location of grenade\nafter 2 second delay
        (Development|PrintString "Spawned Emitter 5")
        (Rendering|SetVisibility (Variables|/Script/Engine.Actor|GetRootComponent _returnvalue_2) false false)
        (for _array_element (Collision|GetOverlappingActors (Variables|Default|GetSphere) "/Game/AI_Blueprints/BP_Enemy_Base.BP_Enemy_Base_C" :!class /Script/Engine.PrimitiveComponent) ; Checks for enemies caught\nin aoe blast
          ;[1 1 1] Halves health of enemy and sets taken health as 'Decay Health', applying that damage to the enemybase
          (bind _asbp_enemy_base (Utilities|Casting|CastToBP_Enemy_Base _array_element)
            (:then
              (Variables|Default|SetHealthBeforeDecay (Variables|/Game/AI_Blueprints/BP_Enemy_Base.BP_Enemy_Base_C|GetHealth _asbp_enemy_base))
              (bind _output_get (Variables|Default|SetDecayHealth (* (Variables|/Game/AI_Blueprints/BP_Enemy_Base.BP_Enemy_Base_C|GetHealth _asbp_enemy_base) 0.5)))
              (bind _returnvalue_3 (Game|Damage|ApplyDamage _asbp_enemy_base _output_get 0 0 "/Script/Engine.DamageType"))
              (Development|PrintString (Utilities|String|ToString(Float) _returnvalue_3) true true "(R=0.000000,G=1.000000,B=0.155471,A=1.000000)")
              (Utilities|FlowControl|Delay 5.0) ; Wait x seconds before adding\nhealth back to enemy
              ;[1 1 1] Checks to make sure enemy is still alive before adding health back
              (CallFunction|CheckHealth)
              (if (Variables|Default|GetAlive?)
                ;[1 1 1] Adds health back slowly
                (if (< (Variables|/Game/AI_Blueprints/BP_Enemy_Base.BP_Enemy_Base_C|GetHealth _asbp_enemy_base) (Variables|Default|GetHealthBeforeDecay)) :!label _label
                  (Variables|/Game/AI_Blueprints/BP_Enemy_Base.BP_Enemy_Base_C|SetHealth _asbp_enemy_base (+ (Variables|/Game/AI_Blueprints/BP_Enemy_Base.BP_Enemy_Base_C|GetHealth _asbp_enemy_base) 0.005))
                  (Utilities|FlowControl|Delay 0.01)
                  (goto _label)
                  (else
                    (Development|PrintString "done adding health")))
                (else
                  (Development|PrintString "Already Dead"))))
            (:CastFailed
              (Development|PrintString "no damage" true true "(R=1.000000,G=0.297888,B=0.000000,A=1.000000)"))))
        (else
          (Development|PrintString "False on Decay Grenade Check 2.5"))))))

(fn ConstructionScript)